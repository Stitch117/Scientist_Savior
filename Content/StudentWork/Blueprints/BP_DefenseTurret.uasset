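; BP_DefenseTurret is a turret that fires projectiles continuously while it is switched on.
; BeginPlay starts a fast looping timer that calls Attack, which spawns BP_Enemy_Projectile_Turret at the Arrow component's location and rotation if ON is true.
; Tick checks the same ON flag every frame and sets the static mesh to a flat black material while the turret is off.
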(event Custom|Attack%20Timer
  ;[1 1 1] Start Attack
  (bind _returnvalue (Utilities|Time|SetTimerbyEvent (delegate Custom|Attack) 0.15 true))
  (Variables|Default|SetAttack%20Timr _returnvalue))

(event Custom|Attack
  (bind _arrow (Variables|Default|GetArrow))
  ;[1 1 1] Spawn bullet
  (if (Variables|Default|GetON?)
    (Game|SpawnActorfromClass "/Game/StudentWork/Blueprints/enemies/BP_Enemy_Projectile_Turret.BP_Enemy_Projectile_Turret_C" (Math|Transform|MakeTransform (Transformation|GetWorldLocation _arrow) (Transformation|GetWorldRotation _arrow) "1.000000,1.000000,1.000000") "Undefined" "MultiplyWithRoot" 0 0)))

(event EventBeginPlay
  (CallFunction|AttackTimer))

(event EventTick
  (params (DeltaSeconds :type Float%20%28single-precision%29))
  ;[1 1 1] Change colour when turned off
  (if (not (Variables|Default|GetON?))
    (Rendering|Material|SetMaterial (Variables|Default|GetStaticMesh) 0 "/Game/Materials/MI_FlatBlack.MI_FlatBlack")))

(fn ConstructionScript)