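; BP_RangedSpider is a ranged enemy that fires BP_SpiderShot projectiles once a player enters its detection sphere.
; The overlap caches the player and starts a looping timer that spawns shots from an arrow's transform, with no logic to stop it.
; Each Tick rotates an arrow component toward the cached player and polls a referenced barrel, destroying the spider after a short delay when that barrel explodes.
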(event OnComponentBeginOverlap(Sphere13)
  (params (OverlappedComponent :type Primitive%20Component%20Object%20Reference) (OtherActor :type Actor%20Object%20Reference) (OtherComp :type Primitive%20Component%20Object%20Reference) (OtherBodyIndex :type Integer) (bFromSweep :type Boolean) (SweepResult :type Hit%20Result%20Structure%20%28by%20ref%29))
  ;[1 1 1] Start Attacking on charachter overlap
  (bind _asbp_player_character (Utilities|Casting|CastToBP_PlayerCharacter OtherActor))
  (Variables|Default|SetAs%20BP%20Player%20Character _asbp_player_character)
  (CallFunction|StartAttackTimer))

(event Custom|Start%20Attack%20Timer
  ;[1 1 1] Start attack timer
  (bind _returnvalue (Utilities|Time|SetTimerbyEvent (delegate Custom|Attack) 0.75 true))
  (Variables|Default|SetSet%20Attack%20Timer _returnvalue))

(event Custom|Attack
  (bind _arrow1 (Variables|Default|GetArrow1))
  (bind _returnvalue (Transformation|GetWorldRotation _arrow1))
  ;[1 1 1] Attack
  (Game|SpawnActorfromClass "/Game/StudentWork/Blueprints/enemies/BP_SpiderShot.BP_SpiderShot_C" (Math|Transform|MakeTransform (Transformation|GetWorldLocation _arrow1) (Math|Rotator|MakeRotator (.roll _returnvalue) (.pitch _returnvalue) (.yaw _returnvalue)) "1.000000,1.000000,1.000000") "Undefined" "MultiplyWithRoot" 0 0))

(event Custom|Look%20at%20player
  (bind _as_bp_player_character (Variables|Default|GetAs%20BP%20Player%20Character))
  (bind _arrow_component (Variables|Default|GetArrow%20Component))
  ;[1 1 1] Look at player
  (Utilities|IsValid _as_bp_player_character
    (:Is%20Valid
      (Transformation|SetWorldRotation _arrow_component (Math|Rotator|FindLookatRotation (Transformation|GetWorldLocation _arrow_component) (Transformation|GetActorLocation _as_bp_player_character)) false false))))

(event Custom|Check%20dead
  ;[1 1 1] Killed when explosion of batrrel goes off
  (if (Variables|/Game/StudentWork/Blueprints/BP_Explosive_Barrel.BP_Explosive_Barrel_C|GetExploding? (Variables|Default|GetBarrel))
    (Utilities|FlowControl|Delay 2.0)
    (Actor|DestroyActor)))

(event EventTick
  (params (DeltaSeconds :type Float%20%28single-precision%29))
  (Utilities|FlowControl|Sequence
    (:then_0
      (CallFunction|LookatPlayer))
    (:then_1
      (CallFunction|CheckDead))))

(fn ConstructionScript)