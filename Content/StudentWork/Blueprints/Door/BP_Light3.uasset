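; BP_Light3 is a door-puzzle Blueprint that activates a third light once three linked spiders are dead.
; Every Tick it checks the Dead flag on all three spider references.
; When all are true, it moves the Light3 actor to its own static mesh's location, clears that light's FunctionedOnce flag, then destroys itself.
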(event EventTick
  (params (DeltaSeconds :type Float%20%28single-precision%29))
  ;[1 1 1] Change the actor to specificall ylight 3 on when all three spdiers are dead
  (if (Math|Boolean|ANDBoolean (Variables|/Game/StudentWork/Blueprints/enemies/BP_ChaserSmall.BP_ChaserSmall_C|GetDead? (Variables|Default|GetSpider1)) (Variables|/Game/StudentWork/Blueprints/enemies/BP_ChaserSmall.BP_ChaserSmall_C|GetDead? (Variables|Default|GetSpider2)) (Variables|/Game/StudentWork/Blueprints/enemies/BP_ChaserSmall.BP_ChaserSmall_C|GetDead? (Variables|Default|GetSpider3)))
    (Transformation|SetActorLocation (Variables|Default|GetLight%203) (Transformation|GetWorldLocation (Variables|Default|GetStaticMesh)) false false)
    (Variables|/Game/StudentWork/Blueprints/Door/BP_Light3On.BP_Light3On_C|SetFunctioned%20Once (Variables|Default|GetLight%203) false)
    (Actor|DestroyActor)))

(fn ConstructionScript)