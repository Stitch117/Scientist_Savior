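; BP_Bomb_AND_Laser_Weapon is a tank weapon with a laser as its primary fire and a bomb as its secondary fire.
; Triggered spawns a stretched laser projectile at the tank's DirectionArrow, and TriggeredSEC spawns a bomb projectile at its BombArrow.
; Each fire mode has its own boolean cooldown, reset after a Delay, with the bomb's lasting longer than the laser's.
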(event EventTriggeredSEC
  (bind _mytank (Variables|Default|GetMyTank))
  (bind _bomb_arrow (Variables|/Game/Blueprints/BP_PlayerCharacter.BP_PlayerCharacter_C|GetBomb%20Arrow _mytank))
  ;[1 1 1] Bomb Shot
  (if (not (Variables|Default|GetBOMB_Cooldown?))
    (Game|SpawnActorfromClass "/Game/StudentWork/Blueprints/Weapons/BP_Bomb_Projectile.BP_Bomb_Projectile_C" (Math|Transform|MakeTransform (Transformation|GetWorldLocation _bomb_arrow) (Transformation|GetWorldRotation _bomb_arrow) "1.000000,1.000000,1.000000") "Undefined" "MultiplyWithRoot" 0 0)
    (Variables|Default|SetBOMB_Cooldown? true)
    (Utilities|FlowControl|Delay 3.0)
    (Variables|Default|SetBOMB_Cooldown? false)))

(event EventTriggered
  (bind _mytank (Variables|Default|GetMyTank))
  (bind _directionarrow (Variables|/Game/Blueprints/BP_PlayerCharacter.BP_PlayerCharacter_C|GetDirectionArrow _mytank))
  ;[1 1 1] Shooting laser
  (if (not (Variables|Default|GetCooldown?))
    (Game|SpawnActorfromClass "/Game/StudentWork/Blueprints/Weapons/BP_LaserProjectile.BP_LaserProjectile_C" (Math|Transform|MakeTransform (Transformation|GetWorldLocation _directionarrow) (Transformation|GetWorldRotation _directionarrow) "3.000000,0.150000,0.150000") "Undefined" "MultiplyWithRoot" 0 0)
    (Variables|Default|SetCooldown? true)
    (Utilities|FlowControl|Delay 0.75)
    (Variables|Default|SetCooldown? false)))

(fn ConstructionScript
  (|CallParentFunction))