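; Spider boss enemy that fires homing shots at the player, deals contact damage through its Cube overlap and calls in minions as health drops.
; Tick checks two one-shot health thresholds, each spawning a pair of BP_Boss_Spawn with effects at hardcoded locations, and uses a Delay to fire from FireArrow about every second.
; Incoming damage is reduced by a flat amount; at zero health it sets both cages moving and destroys itself.
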(event OnComponentBeginOverlap(Cube)
  (params (OverlappedComponent :type Primitive%20Component%20Object%20Reference) (OtherActor :type Actor%20Object%20Reference) (OtherComp :type Primitive%20Component%20Object%20Reference) (OtherBodyIndex :type Integer) (bFromSweep :type Boolean) (SweepResult :type Hit%20Result%20Structure%20%28by%20ref%29))
  ;[1 1 1] Apply damage
  (Game|Damage|ApplyDamage OtherActor 5e+01 0 0))

(event Custom|Spawn%202
  ;[1 1 1] Spider Spawn at 200 health
  (if (<= (Variables|Default|GetCurrent%20Health) 1e+02)
    (if (not (Variables|Default|GetSpawn2))
      (Game|SpawnActorfromClass "/Game/StudentWork/Blueprints/enemies/BP_Boss_Spawn.BP_Boss_Spawn_C" (Math|Transform|MakeTransform "-59564.787033,-522.533441,300.000000" "0, 0, 0" "2.000000,2.000000,2.000000") "Undefined" "MultiplyWithRoot" 0 0)
      (Niagara|SpawnSystematLocation "/Game/StudentWork/Particles/P_BossSpawn.P_BossSpawn" "-59700.469691,-300.000000,1.000000")
      (Game|SpawnActorfromClass "/Game/StudentWork/Blueprints/enemies/BP_Boss_Spawn.BP_Boss_Spawn_C" (Math|Transform|MakeTransform "-59673.177059,-4550.325265,300.000000" "0, 0, 0" "2.000000,2.000000,2.000000") "Undefined" "MultiplyWithRoot" 0 0)
      (Niagara|SpawnSystematLocation "/Game/StudentWork/Particles/P_BossSpawn.P_BossSpawn" "-59789.177059,-4300.000000,1.000000")
      (Variables|Default|SetSpawn2 true))))

(event Custom|Spawn%201
  ;[1 1 1] Spider Spawn at 200 health
  (if (<= (Variables|Default|GetCurrent%20Health) 2e+02)
    (if (not (Variables|Default|Getspawn1))
      (Game|SpawnActorfromClass "/Game/StudentWork/Blueprints/enemies/BP_Boss_Spawn.BP_Boss_Spawn_C" (Math|Transform|MakeTransform "-59564.787033,-522.533441,300.000000" "0, 0, 0" "2.000000,2.000000,2.000000") "Undefined" "MultiplyWithRoot" 0 0)
      (Niagara|SpawnSystematLocation "/Game/StudentWork/Particles/P_BossSpawn.P_BossSpawn" "-59700.469691,-300.000000,1.000000")
      (Game|SpawnActorfromClass "/Game/StudentWork/Blueprints/enemies/BP_Boss_Spawn.BP_Boss_Spawn_C" (Math|Transform|MakeTransform "-59673.177059,-4550.325265,300.000000" "0, 0, 0" "2.000000,2.000000,2.000000") "Undefined" "MultiplyWithRoot" 0 0)
      (Niagara|SpawnSystematLocation "/Game/StudentWork/Particles/P_BossSpawn.P_BossSpawn" "-59789.177059,-4300.000000,1.000000")
      (Variables|Default|Setspawn1 true))))

(event Custom|Attack
  (bind _as_bp_player_character (Variables|Default|GetAs%20BP%20Player%20Character))
  (bind _fire_arrow (Variables|Default|GetFire%20arrow))
  ;[1 1 1] Shoot Homing projectiles
  (bind _returnvalue (Game|SpawnActorfromClass "/Game/StudentWork/Blueprints/enemies/BP_HomingShot.BP_HomingShot_C" (Math|Transform|MakeTransform (Transformation|GetWorldLocation _fire_arrow) (Transformation|GetWorldRotation _fire_arrow) "1.000000,1.000000,1.000000") "Undefined" "MultiplyWithRoot" 0 0))
  (Utilities|IsValid _as_bp_player_character
    (:Is%20Valid
      (Variables|/Script/Engine.ProjectileMovementComponent|SetHomingTargetComponent (Variables|/Game/StudentWork/Blueprints/enemies/BP_HomingShot.BP_HomingShot_C|GetProjectileMovement _returnvalue) (Variables|/Script/Engine.Character|GetCapsuleComponent _as_bp_player_character)))))

(event Game|Damage|EventAnyDamage
  (params (Damage :type Float%20%28single-precision%29) (DamageType :type Damage%20Type%20Object%20Reference) (InstigatedBy :type Controller%20Object%20Reference) (DamageCauser :type Actor%20Object%20Reference))
  ;[1 1 1] health
  (Variables|Default|SetCurrent%20Health (- (Variables|Default|GetCurrent%20Health) (- Damage 7.0)))
  (if (<= (Variables|Default|GetCurrent%20Health) 0.0)
    (Variables|/Game/StudentWork/Blueprints/BP_cage.BP_cage_C|SetMoving? (Variables|Default|GetCage1) true)
    (Variables|/Game/StudentWork/Blueprints/BP_cage.BP_cage_C|SetMoving? (Variables|Default|GetCage2) true)
    (Actor|DestroyActor)))

(event EventTick
  (params (DeltaSeconds :type Float%20%28single-precision%29))
  ;[1 1 1] Check fo rspawning the small ones, and attack on a delay
  (Utilities|FlowControl|Sequence
    (:then_0
      (CallFunction|Spawn1))
    (:then_1
      (CallFunction|Spawn2))
    (:then_2
      (Utilities|FlowControl|Delay 1.0)
      (CallFunction|Attack))))

(fn ConstructionScript
  (|CallParentFunction))