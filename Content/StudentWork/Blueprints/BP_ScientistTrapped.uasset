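; Trapped scientist actor that escapes when its referenced barrel explodes, then leaves rewards for the player.
; Tick watches the barrel's Exploding flag, gated by a Moving bool, then removes the text render and rotates the actor.
; A timeline lerps the static mesh from its start location along a fixed offset.
; When it finishes, the actor turns and spawns a health pack, a bomb weapon pickup and a text actor.
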(event EventTick
  (params (DeltaSeconds :type Float%20%28single-precision%29))
  (bind _start_location (Variables|Default|GetStart%20Location))
  ;[1 1 1] Move the tank if not already moving
  (if (Variables|Default|GetMoving?)
    (if (Variables|/Game/StudentWork/Blueprints/BP_Explosive_Barrel.BP_Explosive_Barrel_C|GetExploding? (Variables|Default|GetBarrel))
      (Components|DestroyComponent (Variables|Default|GetTextRender))
      (Transformation|SetActorRotation "0.000000,110.000000,0.000000")
      (bind _newtrack_0 (Timeline|Timeline Play)
        (:Update
          (Transformation|SetWorldLocation (Variables|Default|GetStaticMesh) (Math|Vector|Lerp(Vector) _start_location (+ _start_location "-1750.000000,3500.000000,0.000000") _newtrack_0) false false)
          (Variables|Default|SetMoving? false))
        (:Finished
          ;[1 1 1] Turn around and spawn collectibles with text after reaching location
          (Transformation|SetActorRotation "0.000000,300.000000,0.000000")
          (Game|SpawnActorfromClass "/Game/StudentWork/Blueprints/BP_Healthpack.BP_Healthpack_C" (Math|Transform|MakeTransform (+ (Transformation|GetActorLocation) "350.000000,0.000000,100.000000") "0.000000,100.000000,0.000000" "4.000000,4.000000,4.000000") "Undefined" "MultiplyWithRoot" 0 0)
          (Game|SpawnActorfromClass "/Game/StudentWork/Blueprints/Weapons/BP_Bomb_Weapon_Pickup.BP_Bomb_Weapon_Pickup_C" (Math|Transform|MakeTransform (+ (Transformation|GetActorLocation) "-200.000000,-200.000000,15.000000") "0, 0, 0" "2.000000,2.000000,2.000000") "Undefined" "MultiplyWithRoot" 0 0)
          (Game|SpawnActorfromClass "/Game/StudentWork/Blueprints/BP_TextForScientist.BP_TextForScientist_C" (Math|Transform|MakeTransform (+ (Transformation|GetActorLocation) "0.000000,0.000000,400.000000") "-15.000000,180.000000,0.000000" "1.000000,1.000000,1.000000") "Undefined" "MultiplyWithRoot" 0 0))))))

(event EventBeginPlay
  ;[1 1 1] get start location
  (Variables|Default|SetStart%20Location (Transformation|GetActorLocation)))

(fn ConstructionScript)