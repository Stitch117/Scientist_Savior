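; BP_ScientistInShip is a scientist pawn that wanders around the navigable area.
; It starts a movement timer on BeginPlay and calls HullToFace every tick, with neither function defined in this file.
; Its Move event sends it by AIMoveTo to a random reachable point within a very large radius, then sets MovementUpdateTime.
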(event EventMove
  ;[1 1 1] Movement
  (AI|AIMoveTo self (.RandomLocation (AI|Navigation|GetRandomReachablePointinRadius (Transformation|GetActorLocation) 1e+06 0 0)) 0 5.0 false
    (:then
      (Variables|Default|SetMovement%20Update%20Time 2.0))))

(event EventBeginPlay
  (CallFunction|StartMovementTimer))

(event EventTick
  (params (DeltaSeconds :type Float%20%28single-precision%29))
  (CallFunction|HulltoFace))

(fn ConstructionScript
  (|CallParentFunction))