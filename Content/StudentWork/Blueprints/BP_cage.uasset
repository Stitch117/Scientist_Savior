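; BP_cage is a cage actor that lowers out of the way, per its comment when the boss dies.
; BeginPlay records the Cube's world location.
; While the Moving flag is true, Tick plays a timeline that lerps the Cube straight down from that start position, without sweeping.
; Nothing in this Blueprint sets Moving.
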(event EventTick
  (params (DeltaSeconds :type Float%20%28single-precision%29))
  (bind _start_location (Variables|Default|GetStart%20Location))
  ;[1 1 1] Moving the cage down when boss is dead
  (if (Variables|Default|GetMoving?)
    (bind _newtrack_0 (Timeline|Timeline Play)
      (:Update
        (Transformation|SetWorldLocation (Variables|Default|GetCube) (Math|Vector|Lerp(Vector) _start_location (+ _start_location "0.000000,0.000000,-610.000000") _newtrack_0) false false)))))

(event EventBeginPlay
  ;[1 1 1] Find start location
  (Variables|Default|SetStart%20Location (Transformation|GetWorldLocation (Variables|Default|GetCube))))

(fn ConstructionScript)