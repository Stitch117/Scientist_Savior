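; BP_Defense_Switch is a switch that shuts down level defenses when the player character touches its box trigger.
; On overlap it clears the ON flag on two referenced turrets and a computer.
; It then redirects guide arrows by swapping their cube materials, hiding some with an invisible translucent material and showing others with the arrow material.
; Nothing in the graph turns the defenses back on or restores the arrows.
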(event OnComponentBeginOverlap(Box)
  (params (OverlappedComponent :type Primitive%20Component%20Object%20Reference) (OtherActor :type Actor%20Object%20Reference) (OtherComp :type Primitive%20Component%20Object%20Reference) (OtherBodyIndex :type Integer) (bFromSweep :type Boolean) (SweepResult :type Hit%20Result%20Structure%20%28by%20ref%29))
  ;[1 1 1] Turn off turrets ad computer when player contact happens
  (bind _asbp_player_character (Utilities|Casting|CastToBP_PlayerCharacter OtherActor))
  (Utilities|IsValid _asbp_player_character
    (:Is%20Valid
      (Variables|/Game/StudentWork/Blueprints/BP_DefenseTurret.BP_DefenseTurret_C|SetON? (Variables|Default|GetTurret) false)
      (Variables|/Game/StudentWork/Blueprints/BP_DefenseTurret.BP_DefenseTurret_C|SetON? (Variables|Default|GetTurret%202) false)
      (Variables|/Game/StudentWork/Blueprints/BP_Defense_Computer.BP_Defense_Computer_C|SetON? (Variables|Default|GetComputer) false)
      ;[1 1 1] Change the arrow directions
      (Rendering|Material|SetMaterial (Variables|/Game/StudentWork/Decale/ArrowCube.ArrowCube_C|GetCube (Variables|Default|GetArrow%201)) 0 "/Engine/Engine_MI_Shaders/Instances/M_Shader_SimpleTranslucent_Invis.M_Shader_SimpleTranslucent_Invis")
      (Rendering|Material|SetMaterial (Variables|/Game/StudentWork/Decale/ArrowCube.ArrowCube_C|GetCube (Variables|Default|GetArrow%202)) 0 "/Engine/Engine_MI_Shaders/Instances/M_Shader_SimpleTranslucent_Invis.M_Shader_SimpleTranslucent_Invis")
      (Rendering|Material|SetMaterial (Variables|/Game/StudentWork/Decale/ArrowCube.ArrowCube_C|GetCube (Variables|Default|GetArrow%203)) 0 "/Engine/Engine_MI_Shaders/Instances/M_Shader_SimpleTranslucent_Invis.M_Shader_SimpleTranslucent_Invis")
      (Rendering|Material|SetMaterial (Variables|/Game/StudentWork/Decale/ArrowOff.ArrowOff_C|GetCube (Variables|Default|GetArrow%207)) 0 "/Game/StudentWork/Decale/Arrow01_Mat.Arrow01_Mat")
      (Rendering|Material|SetMaterial (Variables|/Game/StudentWork/Decale/ArrowOff.ArrowOff_C|GetCube (Variables|Default|GetArrow%208)) 0 "/Game/StudentWork/Decale/Arrow01_Mat.Arrow01_Mat")
      (Rendering|Material|SetMaterial (Variables|/Game/StudentWork/Decale/ArrowOff.ArrowOff_C|GetCube (Variables|Default|GetArrow%209)) 0 "/Game/StudentWork/Decale/Arrow01_Mat.Arrow01_Mat")
      (Rendering|Material|SetMaterial (Variables|/Game/StudentWork/Decale/ArrowOff.ArrowOff_C|GetCube (Variables|Default|GetArrow%2010)) 0 "/Engine/Engine_MI_Shaders/Instances/M_Shader_SimpleTranslucent_Invis.M_Shader_SimpleTranslucent_Invis")
      (Rendering|Material|SetMaterial (Variables|/Game/StudentWork/Decale/ArrowOff.ArrowOff_C|GetCube (Variables|Default|GetArrow%2011)) 0 "/Engine/Engine_MI_Shaders/Instances/M_Shader_SimpleTranslucent_Invis.M_Shader_SimpleTranslucent_Invis")
      (Rendering|Material|SetMaterial (Variables|/Game/StudentWork/Decale/ArrowOff.ArrowOff_C|GetCube (Variables|Default|GetArrow%2012)) 0 "/Engine/Engine_MI_Shaders/Instances/M_Shader_SimpleTranslucent_Invis.M_Shader_SimpleTranslucent_Invis")
      (Rendering|Material|SetMaterial (Variables|/Game/StudentWork/Decale/ArrowOff.ArrowOff_C|GetCube (Variables|Default|GetArrow%2013)) 0 "/Game/StudentWork/Decale/Arrow01_Mat.Arrow01_Mat")
      (Rendering|Material|SetMaterial (Variables|/Game/StudentWork/Decale/ArrowOff.ArrowOff_C|GetCube (Variables|Default|GetArrow%2014)) 0 "/Game/StudentWork/Decale/Arrow01_Mat.Arrow01_Mat")
      (Rendering|Material|SetMaterial (Variables|/Game/StudentWork/Decale/ArrowOff.ArrowOff_C|GetCube (Variables|Default|GetArrow%2015)) 0 "/Game/StudentWork/Decale/Arrow01_Mat.Arrow01_Mat"))))

(fn ConstructionScript)