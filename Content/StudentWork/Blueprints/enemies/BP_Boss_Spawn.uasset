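; Boss spawn enemy pawn with procedurally animated legs that pursues the player character.
; Tick reissues AI Move To toward the stored player reference every frame while it is valid; the reference is not set in this graph.
; A looping timer started on BeginPlay plays three pairs of timelines, each first timeline's update playing the second, to swing six leg pivots by setting their relative rotation.
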(event Custom|CustomEvent
  (Utilities|FlowControl|Sequence
    (:then_0
      (bind _leg1_1 (Timeline|Timeline_4_0 Play)
        (:Update
          (Transformation|SetRelativeRotation (Variables|Default|GetLeg06Pivot) (Math|Rotator|MakeRotator (* _leg1_1 25.0) 0.0 3e+01) false false)
          (bind _leg_2 (Timeline|Timeline_6_0 Play)
            (:Update
              (Transformation|SetRelativeRotation (Variables|Default|GetLeg%204%20Pivot) (Math|Rotator|MakeRotator (* _leg_2 -25.0) 0.0 35.0) false false))))))
    (:then_1
      (bind _leg_3 (Timeline|Timeline_7_0 Play)
        (:Update
          (Transformation|SetRelativeRotation (Variables|Default|Getleg%208%20pivot) (Math|Rotator|MakeRotator (* _leg_3 -25.0) 0.0 -205.0) false false)
          (bind _leg_4 (Timeline|Timeline_8_0 Play)
            (:Update
              (Transformation|SetRelativeRotation (Variables|Default|Getleg%203%20pivot) (Math|Rotator|MakeRotator (* _leg_4 -25.0) 0.0 0.0) false false))))))
    (:then_2
      (bind _newtrack_0 (Timeline|Timeline_9_0 Play)
        (:Update
          (Transformation|SetRelativeRotation (Variables|Default|Getleg%202%20pivot) (Math|Rotator|MakeRotator (* _newtrack_0 -25.0) 0.0 -2e+01) false false)
          (bind _newtrack_0_2 (Timeline|Timeline_10_0 Play)
            (:Update
              (Transformation|SetRelativeRotation (Variables|Default|GetLeg%207%20pivot) (Math|Rotator|MakeRotator (* _newtrack_0_2 25.0) 0.0 0.0) false false))))))))

(event EventBeginPlay
  (bind _returnvalue (Utilities|Time|SetTimerbyEvent (delegate Custom|CustomEvent) 0.1 true))
  (Variables|Default|Setanimation%20timer _returnvalue))

(event EventTick
  (params (DeltaSeconds :type Float%20%28single-precision%29))
  (bind _as_bp_player_character (Variables|Default|GetAs%20BP%20Player%20Character))
  ;[1 1 1] move towards the player
  (Utilities|IsValid _as_bp_player_character
    (:Is%20Valid
      (AI|AIMoveTo self "0, 0, 0" _as_bp_player_character 5.0 false))))

(fn ConstructionScript
  (|CallParentFunction))