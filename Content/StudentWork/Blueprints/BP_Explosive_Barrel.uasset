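; BP_Explosive_Barrel is an explosive barrel actor that starts a one-time fuse when it takes any damage.
; The first hit sets Moving on its Scientist reference, changes the barrel's material and spawns a fuse effect above it.
; After a short delay it spawns a scaled-up BP_ExplosveBarrelDamage actor at its location, then destroys itself.
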(event Game|Damage|EventAnyDamage
  (params (Damage :type Float%20%28single-precision%29) (DamageType :type Damage%20Type%20Object%20Reference) (InstigatedBy :type Controller%20Object%20Reference) (DamageCauser :type Actor%20Object%20Reference))
  (bind _returnvalue (Transformation|GetActorLocation))
  (if (not (Variables|Default|GetExploding?))
    (Variables|/Game/StudentWork/Blueprints/BP_ScientistTrapped.BP_ScientistTrapped_C|SetMoving? (Variables|Default|GetScientist) true)
    (Variables|Default|SetExploding? true)
    (Rendering|Material|SetMaterial (Variables|Default|GetStaticMesh) 0 "/Game/StudentWork/Materials/M_Explosive_barrel.M_Explosive_barrel")
    (Niagara|SpawnSystematLocation "/Game/StudentWork/Particles/P_Target_Fuse.P_Target_Fuse" (Math|Vector|MakeVector (.x _returnvalue) (.y _returnvalue) (+ (.z _returnvalue) 3e+02)))
    (Utilities|FlowControl|Delay 2.0)
    (Game|SpawnActorfromClass "/Game/StudentWork/Blueprints/BP_ExplosveBarrelDamage.BP_ExplosveBarrelDamage_C" (Math|Transform|MakeTransform (Transformation|GetActorLocation) "0, 0, 0" "4.500000,4.500000,4.500000") "Undefined" "MultiplyWithRoot" 0 0)
    (Actor|DestroyActor)))

(fn ConstructionScript)