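; BP_Door1 is a door that slides sideways once its Moving flag is set, noted as when light three is on.
; BeginPlay caches the static mesh's world location as the start point.
; Tick checks Moving and plays a timeline whose alpha lerps the mesh along negative world Y to a fixed offset.
; Nothing in this Blueprint sets Moving or reverses the slide.
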(event EventTick
  (params (DeltaSeconds :type Float%20%28single-precision%29))
  (bind _start_location (Variables|Default|GetStart%20Location))
  ;[1 1 1] Move when light three on
  (if (Variables|Default|GetMoving?)
    (bind _alpha (Timeline|Timeline Play)
      (:Update
        (Transformation|SetWorldLocation (Variables|Default|GetStaticMesh) (Math|Vector|Lerp(Vector) _start_location (+ _start_location "0.000000,-575.000000,0.000000") _alpha) false false)))))

(event EventBeginPlay
  ;[1 1 1] Find start location
  (Variables|Default|SetStart%20Location (Transformation|GetWorldLocation (Variables|Default|GetStaticMesh))))

(fn ConstructionScript)