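; BP_Broken_Turret is an enemy turret that sprays projectiles in random directions and is destroyed when damage depletes its health.
; A player entering its sphere trigger starts a fast looping timer, with no logic to stop it when the player leaves.
; Each tick of that timer spawns a scaled-down BP_Enemy_Projectile_Turret at the arrow component's location with random yaw, so shots are never aimed at the player.
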(event OnComponentBeginOverlap(Sphere)
  (params (OverlappedComponent :type Primitive%20Component%20Object%20Reference) (OtherActor :type Actor%20Object%20Reference) (OtherComp :type Primitive%20Component%20Object%20Reference) (OtherBodyIndex :type Integer) (bFromSweep :type Boolean) (SweepResult :type Hit%20Result%20Structure%20%28by%20ref%29))
  ;[1 1 1] start attacking when overlaping the collision detection with the player
  (bind _asbp_player_character (Utilities|Casting|CastToBP_PlayerCharacter OtherActor))
  (Variables|Default|SetAs%20BP%20Player%20Character _asbp_player_character)
  (CallFunction|StartAttackTimer))

(event Custom|Start%20Attack%20Timer
  ;[1 1 1] Start attcking
  (bind _returnvalue (Utilities|Time|SetTimerbyEvent (delegate Custom|Attack) 0.35 true))
  (Variables|Default|SetAttack%20Timer _returnvalue))

(event Custom|Attack
  ;[1 1 1] Start attcking
  ;[1 1 1] Attacking
  (Game|SpawnActorfromClass "/Game/StudentWork/Blueprints/enemies/BP_Enemy_Projectile_Turret.BP_Enemy_Projectile_Turret_C" (Math|Transform|MakeTransform (Transformation|GetWorldLocation (Variables|Default|GetArrow1)) (Math|Rotator|MakeRotator 0.0 0.0 (.yaw (Math|Random|RandomRotator false))) "0.750000,0.750000,0.750000") "Undefined" "MultiplyWithRoot" 0 0))

(event Game|Damage|EventAnyDamage
  (params (Damage :type Float%20%28single-precision%29) (DamageType :type Damage%20Type%20Object%20Reference) (InstigatedBy :type Controller%20Object%20Reference) (DamageCauser :type Actor%20Object%20Reference))
  ;[1 1 1] health and destroy on death
  (Variables|Default|SetHealth (- (Variables|Default|GetHealth) Damage))
  (if (<= (Variables|Default|GetHealth) 0.0)
    (Actor|DestroyActor)))

(fn ConstructionScript)