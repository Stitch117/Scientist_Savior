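; BP_ChaserSmall is a small spider enemy that hurts what it touches and can be killed.
; A Cube component acts as the front hitbox, applying fixed damage to any overlapping actor without filtering for the player.
; Incoming damage reduces CurrentHealth; at zero it sets Dead and moves the actor to a hardcoded far-off location instead of destroying it.
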(event OnComponentBeginOverlap(Cube)
  (params (OverlappedComponent :type Primitive%20Component%20Object%20Reference) (OtherActor :type Actor%20Object%20Reference) (OtherComp :type Primitive%20Component%20Object%20Reference) (OtherBodyIndex :type Integer) (bFromSweep :type Boolean) (SweepResult :type Hit%20Result%20Structure%20%28by%20ref%29))
  ;[1 1 1] Do damage when player is infront of the spider
  (Game|Damage|ApplyDamage OtherActor 3e+01 0 0))

(event EventBeginPlay
  (Variables|Default|SetDead? false))

(event Game|Damage|EventAnyDamage
  (params (Damage :type Float%20%28single-precision%29) (DamageType :type Damage%20Type%20Object%20Reference) (InstigatedBy :type Controller%20Object%20Reference) (DamageCauser :type Actor%20Object%20Reference))
  ;[1 1 1] health
  (Variables|Default|SetCurrent%20Health (- (Variables|Default|GetCurrent%20Health) Damage))
  (if (<= (Variables|Default|GetCurrent%20Health) 0.0)
    (Variables|Default|SetDead? true)
    (Transformation|SetActorLocation "-69587.201187,41097.549976,3009.191399" false false)))

(fn ConstructionScript
  (|CallParentFunction))