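; Laser weapon for a tank that fires a laser projectile when triggered.
; Each shot spawns BP_LaserProjectile at the world location and rotation of the owning tank's direction arrow, scaled into a long, thin beam shape.
; A Cooldown flag and a short Delay limit the fire rate by ignoring triggers until the delay ends.
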(event EventTriggered
  (bind _mytank (Variables|Default|GetMyTank))
  (bind _directionarrow (Variables|/Game/Blueprints/BP_PlayerCharacter.BP_PlayerCharacter_C|GetDirectionArrow _mytank))
  ;[1 1 1] Shooting
  (if (not (Variables|Default|GetCooldown?))
    (Game|SpawnActorfromClass "/Game/StudentWork/Blueprints/Weapons/BP_LaserProjectile.BP_LaserProjectile_C" (Math|Transform|MakeTransform (Transformation|GetWorldLocation _directionarrow) (Transformation|GetWorldRotation _directionarrow) "3.000000,0.150000,0.150000") "Undefined" "MultiplyWithRoot" 0 0)
    (Variables|Default|SetCooldown? true)
    (Utilities|FlowControl|Delay 0.75)
    (Variables|Default|SetCooldown? false)))

(fn ConstructionScript
  (|CallParentFunction))