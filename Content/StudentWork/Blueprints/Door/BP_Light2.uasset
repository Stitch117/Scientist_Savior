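; BP_Light2 is a door indicator light that turns green once any two of three referenced spiders are dead.
; Every Tick it checks the Dead flag on each pair of spiders.
; When a pair is dead, it spawns BP_Light2On at its static mesh's world transform and destroys itself, swapping actors rather than changing the light in place.
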(event EventTick
  (params (DeltaSeconds :type Float%20%28single-precision%29))
  (bind _spider1 (Variables|Default|GetSpider1))
  (bind _spider2 (Variables|Default|GetSpider2))
  (bind _spider3 (Variables|Default|GetSpider3))
  (bind _dead_ (Variables|/Game/StudentWork/Blueprints/enemies/BP_ChaserSmall.BP_ChaserSmall_C|GetDead? _spider1))
  (bind _dead__2 (Variables|/Game/StudentWork/Blueprints/enemies/BP_ChaserSmall.BP_ChaserSmall_C|GetDead? _spider2))
  (bind _dead__3 (Variables|/Game/StudentWork/Blueprints/enemies/BP_ChaserSmall.BP_ChaserSmall_C|GetDead? _spider3))
  ;[1 1 1] Change the light to a green one when any 2 of the spiders are dead
  (if (Math|Boolean|ORBoolean (and _dead_ _dead__2) (and _dead_ _dead__3) (and _dead__2 _dead__3))
    (Game|SpawnActorfromClass "/Game/StudentWork/Blueprints/Door/BP_Light2On.BP_Light2On_C" (Transformation|GetWorldTransform (Variables|Default|GetStaticMesh)) "Undefined" "MultiplyWithRoot" 0 0)
    (Actor|DestroyActor)))

(fn ConstructionScript)