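; BP_Light1 is a door indicator light actor that switches to its lit version once any one of three referenced spiders dies.
; Each tick it polls the Dead flag on the three spider references.
; When one is set, it spawns BP_Light1On at its static mesh's transform and destroys itself, swapping actors instead of changing material.
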(event EventTick
  (params (DeltaSeconds :type Float%20%28single-precision%29))
  ;[1 1 1] Change the actor to a green one when any one of the three spiders died
  (if (Math|Boolean|ORBoolean (Variables|/Game/StudentWork/Blueprints/enemies/BP_ChaserSmall.BP_ChaserSmall_C|GetDead? (Variables|Default|GetSpider1)) (Variables|/Game/StudentWork/Blueprints/enemies/BP_ChaserSmall.BP_ChaserSmall_C|GetDead? (Variables|Default|GetSpider2)) (Variables|/Game/StudentWork/Blueprints/enemies/BP_ChaserSmall.BP_ChaserSmall_C|GetDead? (Variables|Default|GetSpider3)))
    (Game|SpawnActorfromClass "/Game/StudentWork/Blueprints/Door/BP_Light1On.BP_Light1On_C" (Transformation|GetWorldTransform (Variables|Default|GetStaticMesh)) "Undefined" "MultiplyWithRoot" 0 0)
    (Actor|DestroyActor)))

(fn ConstructionScript)